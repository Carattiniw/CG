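; Game mode for a gamepad menu that keeps a running score, with UpdateScore adding each note's score to the current total.
; BeginPlay calls SetMusic, but that function is empty because its body is disconnected.
; The unconnected logic would play the player's music track from an accumulated pause offset or stop it, using the gamepad controller's music timer.
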(event `self.ReceiveBeginPlay`
  (`self.SetMusic` true))

(fn `SetMusic`
  (params (`Play?` :type Boolean)))

(fn `UpdateScore`
  (params (`Note Score` :type Integer))
  ;[1 1 1] Add to current score; keeps value updated
  (set `self.CurrentScore` (+ `Note Score` (`self.CurrentScore`))))

(fn `UserConstructionScript`)