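; Left fret trigger zone for a rhythm-style game, letting the player hit BP_LeftTarget notes for points.
; A note overlapping the actor enables input and opens a gate, and a note leaving disables input and closes it.
; Pressing Z while the gate is open destroys the cast target references and passes NoteValue to UpdateScore on ThirdPersonGameMode.
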(event `Key|Z`
  (params (Key :type "Key Structure"))
  ;[1 1 1] Enable or disable input accordingly
  (:`Pressed`
    (`/Engine/EditorBlueprintResources/StandardMacros.Gate` true :!label _label ; Only proceed if corresponding note is inside trigger zone and the player presses the appropriate input
      (:`Exit`
        ;[1 1 1] Destroy note from scene and update score
        (`self.K2_DestroyActor` (stale `self.ReceiveActorBeginOverlap` _asbp_left_target))
        (`self.K2_DestroyActor` (stale `self.ReceiveActorEndOverlap` _asbp_left_target))
        (bind _asthird_person_game_mode (cast `/Game/ThirdPersonBP/Blueprints/ThirdPersonGameMode` (`GameplayStatics.GetGameMode`)))
        (`/Game/ThirdPersonBP/Blueprints/ThirdPersonGameMode.UpdateScore` _asthird_person_game_mode (`self.Note Value`))))))

(event `self.ReceiveActorBeginOverlap`
  (params (OtherActor :type "Actor Object Reference"))
  ;[1 1 1] Check to see if a "note" is within trigger zone ("fret")
  (bind _asbp_left_target (cast `/Game/Blueprints/BP_Notes/BP_LeftTarget` OtherActor))
  ;[1 1 1] Enable or disable input accordingly
  (`self.EnableInput` (`GameplayStatics.GetPlayerController` 0))
  (goto _label :!via `Open`))

(event `self.ReceiveActorEndOverlap`
  (params (OtherActor :type "Actor Object Reference"))
  ;[1 1 1] Check to see if a "note" is within trigger zone ("fret")
  (bind _asbp_left_target (cast `/Game/Blueprints/BP_Notes/BP_LeftTarget` OtherActor))
  ;[1 1 1] Enable or disable input accordingly
  (`self.DisableInput` (`GameplayStatics.GetPlayerController` 0))
  (goto _label :!via `Close`))

(fn `UserConstructionScript`)