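; BP_GamePadPC is a player controller that runs the pause menu, creating PauseMenu_UI at BeginPlay.
; The Menu input toggles OpenMenu and CloseMenu, switching widget, input mode, cursor and game pause, toggling GM_GamePadMenu music, and calling the player's SetMovement(false) both ways.
; StopPauseMenu and AllowPauseMenu set an OnMainMenu flag that blocks the toggle on the main menu.
; Two music timer events record audio start and pause times.
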(event `self.ReceiveBeginPlay`
  ;[1 1 1] Cast pause menu widget to screen (behavior controlled by "Main Pause Menu" below)
  (bind _returnvalue (`|CreateWidget` "/Game/Blueprints/PauseMenu_UI.PauseMenu_UI_C"))
  (set `self.MainMenu` _returnvalue)
  (set `self.PlayerCharacter` (cast `/Game/Blueprints/BP_TestPlayer` (`self.K2_GetPawn`) :!pure true)))

(event `InputAction|Menu` :paused true
  (params (Key :type "Key Structure"))
  ;[1 1 1] Main Pause Menu
  ;;[1 1 1] Detects if pause button was pressed
  (:`Pressed`
    ;;;[1 1 1] Stops pause menu from appearing on main menu
    (if (`self.OnMainMenu?`)
      _
      (elif (`self.MenuOpened?`)
        (`self.CloseMenu`)
        (else
          (`self.OpenMenu`))))))

(event `CloseMenu`
  ;[1 1 1] Main Pause Menu
  ;;[1 1 1] Closes Menu
  (`Widget.RemoveFromParent` (`self.MainMenu`))
  (`WidgetBlueprintLibrary.SetInputMode_GameOnly` self)
  ;;;[1 1 1] Resumes music when unpaused
  (bind _asgm_game_pad_menu (cast `/Game/Blueprints/GM_GamePadMenu` (`GameplayStatics.GetGameMode`)))
  (`/Game/Blueprints/GM_GamePadMenu.SetMusic` _asgm_game_pad_menu true)
  (set `self.bShowMouseCursor` false)
  (set `self.MenuOpened?` false)
  (`/Game/Blueprints/BP_TestPlayer.SetMovement` (`self.PlayerCharacter`) false)
  (`GameplayStatics.SetGamePaused` false))

(event `OpenMenu`
  (bind _mainmenu (`self.MainMenu`))
  ;[1 1 1] Main Pause Menu
  ;;[1 1 1] Open Menu
  (`UserWidget.AddToViewport` _mainmenu 0)
  (`WidgetBlueprintLibrary.SetInputMode_GameAndUIEx` self _mainmenu)
  ;;;[1 1 1] Stops music when paused
  (bind _asgm_game_pad_menu (cast `/Game/Blueprints/GM_GamePadMenu` (`GameplayStatics.GetGameMode`)))
  (`/Game/Blueprints/GM_GamePadMenu.SetMusic` _asgm_game_pad_menu false)
  (set `self.bShowMouseCursor` true)
  (set `self.MenuOpened?` true)
  (`/Game/Blueprints/BP_TestPlayer.SetMovement` (`self.PlayerCharacter`) false)
  (`GameplayStatics.SetGamePaused` true))

(event `PauseMusicTimer`
  ;[1 1 1] Pause/Resume Music Event Behavior
  (set `self.MusicPausedAt` (`GameplayStatics.GetAudioTimeSeconds`)))

(event `StopPauseMenu`
  ;[1 1 1] Does not allow pause menu to appear.
  ; Allow Pause Menu event must be called on every other level in order for pause menu to work.
  (set `self.OnMainMenu?` true))

(event `StartMusicTimer`
  ;[1 1 1] Pause/Resume Music Event Behavior
  (set `self.MusicStartedAt` (`GameplayStatics.GetAudioTimeSeconds`)))

(event `AllowPauseMenu`
  ;[1 1 1] Does not allow pause menu to appear.
  ; Allow Pause Menu event must be called on every other level in order for pause menu to work.
  (set `self.OnMainMenu?` false))

(fn `UserConstructionScript`)