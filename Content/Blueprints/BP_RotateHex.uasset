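; BP_RotateHex is an actor whose static mesh spins in yaw every tick, optionally starting from a random orientation.
; When ActiveCart is set, it also rides TracRef's spline after a start delay.
; The CartMover timeline, scaled by Duration and started at an offset, lerps spline distance to set location and rotation.
; Delays chained from the timeline's Update and Finished outputs reverse and restart the ride.
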(event `self.ReceiveTick`
  (params (DeltaSeconds :type "Float (single-precision)"))
  ;[1 1 1] Rotates Object
  (`SceneComponent.K2_AddRelativeRotation` (`self.StaticMesh`) (`KismetMathLibrary.MakeRotator` 0.0 0.0 (`self.Rotate Speed`)) false false))

(event `self.ReceiveBeginPlay`
  ;[1 1 1] Move object along spline path
  (`|ExecutionSequence`
    (:`then_0`
      (if (`self.ActiveCart`)
        (`self.MoveCart`)))
    (:`then_1`
      ;[1 1 1] If true, randomizes the orientation of the object
      (if (`self.RandomRotate`)
        (`SceneComponent.K2_AddRelativeRotation` (`self.StaticMesh`) (`KismetMathLibrary.RandomRotator` false) false false)))))

(event `MoveCart`
  (bind _returnvalue (`KismetMathLibrary.Lerp` 0.0 (`SplineComponent.GetSplineLength` (`/Game/Blueprints/BP_SplinePath.UsefulSpline` (`self.TracRef`))) (`self.Alpha`)))
  ;[1 1 1] Move object along spline path
  (`KismetSystemLibrary.Delay` (`self.DelayStartMovement`))
  (`TimelineComponent.SetPlayRate` (`self.CartMover`) (/ 1.0 (`self.Duration`)))
  (`TimelineComponent.SetNewTime` (`self.CartMover`) (`self.KartStartOffset`))
  (bind (_direction _alpha) (`Timeline|CartMover` :!label _label)
    (:`Update`
      (set `self.Alpha` _alpha)
      ;;[1 1 1] Sets the location and rotation of the player character during the ride
      (`self.K2_SetActorLocationAndRotation` (`SplineComponent.GetLocationAtDistanceAlongSpline` (`/Game/Blueprints/BP_SplinePath.UsefulSpline` (`self.TracRef`)) _returnvalue "World") (`SplineComponent.GetRotationAtDistanceAlongSpline` (`/Game/Blueprints/BP_SplinePath.UsefulSpline` (`self.TracRef`)) _returnvalue "World"))
      (`KismetSystemLibrary.Delay` (`self.Duration`))
      (goto _label :!via `ReverseFromEnd`))
    (:`Finished`
      (`KismetSystemLibrary.Delay` (* (`self.Duration`) 2.0))
      (goto _label :!via `PlayFromStart`))))

(fn `UserConstructionScript`)