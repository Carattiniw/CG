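; BP_MovePCAlongPath is a spline path actor that constrains the third-person player character to its curve.
; BeginPlay repositions and rotates the End trigger against the spline and caches the player.
; Player overlap with either Begin or End snaps the capsule on and sets path state; other actors' overlaps clear it.
; While active, Tick pins X and Y to the closest spline point, leaving Z free.
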(event `self.ReceiveBeginPlay`
  (bind _end (`self.End`))
  (bind _spline (`self.Spline`))
  ;[1 1 1] Begin Play Behavior
  (`SceneComponent.K2_SetWorldLocation` _end (`KismetMathLibrary.MakeVector` (+ (.x (`SplineComponent.FindLocationClosestToWorldLocation` (`self.Spline`) (`SceneComponent.K2_GetComponentLocation` (`self.End`)) "Local")) 50.0) (.y (`SplineComponent.FindLocationClosestToWorldLocation` (`self.Spline`) (`SceneComponent.K2_GetComponentLocation` (`self.End`)) "Local")) (.z (`SplineComponent.FindLocationClosestToWorldLocation` (`self.Spline`) (`SceneComponent.K2_GetComponentLocation` (`self.End`)) "Local"))) false false)
  (`SceneComponent.K2_SetWorldRotation` _end (`SplineComponent.GetRotationAtSplinePoint` _spline (`SplineComponent.GetNumberOfSplinePoints` _spline) "Local") false false)
  (bind _asthird_person_character (cast `/Game/ThirdPersonBP/Blueprints/ThirdPersonCharacter` (`GameplayStatics.GetPlayerCharacter` 0)))
  (set `self.PlayerRef` _asthird_person_character))

(event `BeginSpline`
  (bind _playerref (`self.PlayerRef`))
  ;[1 1 1] Begin and End Spline
  (`KismetSystemLibrary.PrintString` "Hello")
  (set `/Game/ThirdPersonBP/Blueprints/ThirdPersonCharacter.InSpline` true _playerref)
  (set `/Game/ThirdPersonBP/Blueprints/ThirdPersonCharacter.PlayerPathRef` self _playerref)
  (`SceneComponent.K2_SetWorldLocation` (`Character.CapsuleComponent` (`self.PlayerRef`)) (`SplineComponent.FindLocationClosestToWorldLocation` (`self.Spline`) (`SceneComponent.K2_GetComponentLocation` (`Character.CapsuleComponent` (`self.PlayerRef`))) "Local") false false)
  (set `self.StartTick` true))

(event `self.ReceiveTick`
  (params (DeltaSeconds :type "Float (single-precision)"))
  (bind _returnvalue (`SceneComponent.K2_GetComponentLocation` (`Character.CapsuleComponent` (`self.PlayerRef`))))
  (bind (_returnvalue_x _returnvalue_y) (`KismetMathLibrary.BreakVector` (`SplineComponent.FindLocationClosestToWorldLocation` (`self.Spline`) _returnvalue "Local")))
  (if (`self.StartTick`)
    (`SceneComponent.K2_SetWorldLocation` (`Character.CapsuleComponent` (`self.PlayerRef`)) (`KismetMathLibrary.MakeVector` _returnvalue_x _returnvalue_y (.z _returnvalue)) false false)))

(event `EndSpline`
  (bind _playerref (`self.PlayerRef`))
  ;[1 1 1] Begin and End Spline
  (set `/Game/ThirdPersonBP/Blueprints/ThirdPersonCharacter.InSpline` false _playerref)
  (set `/Game/ThirdPersonBP/Blueprints/ThirdPersonCharacter.PlayerPathRef` null _playerref)
  (set `self.StartTick` false))

(event `self.Begin.OnComponentBeginOverlap`
  (params (OverlappedComponent :type "PrimitiveComponent Object Reference") (OtherActor :type "Actor Object Reference") (OtherComp :type "PrimitiveComponent Object Reference") (OtherBodyIndex :type Integer) (bFromSweep :type Boolean) (SweepResult :type "HitResult Structure (by ref)"))
  (if (== OtherActor (`self.PlayerRef`))
    (`self.BeginSpline`)
    (else
      (`self.EndSpline`))))

(event `self.End.OnComponentBeginOverlap`
  (params (OverlappedComponent :type "PrimitiveComponent Object Reference") (OtherActor :type "Actor Object Reference") (OtherComp :type "PrimitiveComponent Object Reference") (OtherBodyIndex :type Integer) (bFromSweep :type Boolean) (SweepResult :type "HitResult Structure (by ref)"))
  (if (== OtherActor (`self.PlayerRef`))
    (`self.BeginSpline`)
    (else
      (`self.EndSpline`))))

(fn `UserConstructionScript`)